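; Quest prop backpack that the third-person character collects by walking into it.
; On first overlap it sets the Bckpck flag in SinglePlayerGameInstance, plays a 2D sound, notifies MyGameStat through BackpackCollected and destroys itself.
; BeginPlay and the BckCollect event share a check that removes the actor when that flag is already set, so a collected backpack stays gone.
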(event Custom|BckCollect
  (bind _assingle_player_game_instance (Utilities|Casting|CastToSinglePlayerGameInstance (Game|GetGameInstance)))
  (if (Variables|/Game/SinglePlayerGameInstance.SinglePlayerGameInstance_C|Getbckpck _assingle_player_game_instance)
    (Variables|/Game/SinglePlayerGameInstance.SinglePlayerGameInstance_C|Setbckpck _assingle_player_game_instance true)
    (Actor|DestroyActor)))

(event EventBeginPlay
  (bind _assingle_player_game_instance (Utilities|Casting|CastToSinglePlayerGameInstance (Game|GetGameInstance)))
  (if (Variables|/Game/SinglePlayerGameInstance.SinglePlayerGameInstance_C|Getbckpck _assingle_player_game_instance)
    (Variables|/Game/SinglePlayerGameInstance.SinglePlayerGameInstance_C|Setbckpck _assingle_player_game_instance true)
    (Actor|DestroyActor)))

(event Collision|EventActorBeginOverlap
  (params (OtherActor :type Actor%20Object%20Reference))
  (Utilities|Casting|CastToThirdPersonCharacter OtherActor)
  (bind _assingle_player_game_instance (Utilities|Casting|CastToSinglePlayerGameInstance (Game|GetGameInstance)))
  (if (not (Variables|/Game/SinglePlayerGameInstance.SinglePlayerGameInstance_C|Getbckpck _assingle_player_game_instance))
    (Variables|/Game/SinglePlayerGameInstance.SinglePlayerGameInstance_C|Setbckpck _assingle_player_game_instance true)
    (Audio|PlaySound2D "/Game/Audio/SoundEffects/FlowerCollectSound.FlowerCollectSound" 1.0 1.0 0.0 0 0)
    (bind _asmy_game_stat (Utilities|Casting|CastToMyGameStat (Game|GetGameState)))
    (Default|CallBackpackCollected _asmy_game_stat self)
    (Actor|DestroyActor)))

(fn ConstructionScript)