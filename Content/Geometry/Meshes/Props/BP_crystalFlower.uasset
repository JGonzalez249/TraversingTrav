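; Collectible crystal flower prop that advances Adrogad's dialogue and opens the path behind them when overlapped.
; On overlap, if Adrogad's DKResponse is Case_0 or Case_1, it sets it to Case_2 and destroys the AdroBarrier actor.
; Only afterwards does it cast the overlapping actor to ThirdPersonCharacter, which gates just the flower's destruction and collect sound.
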(event EventBeginPlay)

(event Collision|EventActorBeginOverlap
  (params (OtherActor :type Actor%20Object%20Reference))
  ;[1 1 1] This changes Adrogad's Dialogue
  (bind _returnvalue (Actor|GetActorOfClass "/Game/NPC/PF_FL_Adrogad1.PF_FL_Adrogad1_C"))
  (bind _output_get (Variables|Default|SetAdro _returnvalue))
  (if (or (Utilities|Name|Equal(Name) (Variables|/Game/NPC/DK_NPC.DK_NPC_C|GetDK_Response _output_get) "Case_0") (Utilities|Name|Equal(Name) (Variables|/Game/NPC/DK_NPC.DK_NPC_C|GetDK_Response _output_get) "Case_1"))
    (bind _returnvalue_2 (Actor|GetActorOfClass "/Game/NPC/PF_FL_Adrogad1.PF_FL_Adrogad1_C"))
    (bind _output_get_2 (Variables|Default|SetAdro _returnvalue_2))
    (Variables|/Game/NPC/DK_NPC.DK_NPC_C|SetDK_Response _output_get_2 "Case_2")
    ;[1 1 1] Destroys the invisible barrier behind Adrogad
    (bind _returnvalue_3 (Actor|GetActorOfClass "/Game/NPC/Invisiwall/PF_AdroBarrier.PF_AdroBarrier_C"))
    (Actor|DestroyActor _returnvalue_3)
    ;[1 1 1] This makes the flower disappear
    (Utilities|Casting|CastToThirdPersonCharacter OtherActor)
    (Actor|DestroyActor)
    (Audio|PlaySound2D "/Game/Audio/SoundEffects/FlowerCollectSound.FlowerCollectSound" 1.0 1.0 0.0 0 0)))

(event EventTick
  (params (DeltaSeconds :type Float%20%28single-precision%29)))

(fn ConstructionScript)