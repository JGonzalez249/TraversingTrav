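; Wind zone Blueprint actor that pushes the player's third-person character along the direction of its Arrow component.
; On BeginPlay it caches player 0's character; overlapping the WindZone component starts a looping timer that repeatedly launches that character, adding to its existing velocity, and ending the overlap clears the timer.
; The overlapping actor is never checked, so any overlap pushes the player.
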(event OnComponentBeginOverlap(WindZone)
  (params (OverlappedComponent :type Primitive%20Component%20Object%20Reference) (OtherActor :type Actor%20Object%20Reference) (OtherComp :type Primitive%20Component%20Object%20Reference) (OtherBodyIndex :type Integer) (bFromSweep :type Boolean) (SweepResult :type Hit%20Result%20Structure%20%28by%20ref%29))
  (bind _returnvalue (Utilities|Time|SetTimerbyEvent (delegate Custom|Tick30) 0.2 true)))

(event OnComponentEndOverlap(WindZone)
  (params (OverlappedComponent :type Primitive%20Component%20Object%20Reference) (OtherActor :type Actor%20Object%20Reference) (OtherComp :type Primitive%20Component%20Object%20Reference) (OtherBodyIndex :type Integer))
  (Utilities|Time|ClearandInvalidateTimerbyHandle (stale OnComponentBeginOverlap(WindZone) _returnvalue)))

(event Custom|Tick30
  (Character|LaunchCharacter (Variables|Default|GetChar) (* (Math|Vector|GetForwardVector (Variables|Default|GetArrow)) 5.5e+02) false false))

(event EventBeginPlay
  (bind _asthird_person_character (Utilities|Casting|CastToThirdPersonCharacter (Game|GetPlayerCharacter 0)))
  (Variables|Default|SetChar _asthird_person_character))

(event Collision|EventActorBeginOverlap
  (params (OtherActor :type Actor%20Object%20Reference)))

(event EventTick
  (params (DeltaSeconds :type Float%20%28single-precision%29)))

(fn ConstructionScript)