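; Wind volume actor that pushes physics objects inside its Range box, which the construction script sizes and raises from the range variables.
; While anything overlaps the box, Tick fires a grid of line traces along the actor's up axis.
; Each hit on a simulating component adds force at the impact point, blending up vector and inverted normal, scaled by their alignment.
; The player launch logic is disconnected.
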(event OnComponentBeginOverlap(Range)
  (params (OverlappedComponent :type Primitive%20Component%20Object%20Reference) (OtherActor :type Actor%20Object%20Reference) (OtherComp :type Primitive%20Component%20Object%20Reference) (OtherBodyIndex :type Integer) (bFromSweep :type Boolean) (SweepResult :type Hit%20Result%20Structure%20%28by%20ref%29))
  ;[1 1 1] (Disabled for now) These pieces of code affect the player in regards to wind, player is "flying" and sprinting doesn't do anything when player is in the wind.
)

(event OnComponentEndOverlap(Range)
  (params (OverlappedComponent :type Primitive%20Component%20Object%20Reference) (OtherActor :type Actor%20Object%20Reference) (OtherComp :type Primitive%20Component%20Object%20Reference) (OtherBodyIndex :type Integer))
  ;[1 1 1] (Disabled for now) These pieces of code affect the player in regards to wind, player is "flying" and sprinting doesn't do anything when player is in the wind.
)

(event Custom|Tick30
  ;[1 1 1] (Disabled for now) These pieces of code affect the player in regards to wind, player is "flying" and sprinting doesn't do anything when player is in the wind.
)

(event EventTick
  (params (DeltaSeconds :type Float%20%28single-precision%29))
  (bind _returnvalue (Transformation|GetActorTransform))
  (bind _returnvalue_2 (Transformation|GetActorUpVector))
  (bind _distancebetweenforcelines (Variables|Default|GetDistanceBetweenForceLines))
  (if (> (Utilities|Array|Length (Class|PrimitiveComponent|GetOverlappingComponents (Variables|Default|GetRange))) 0)
    (for _index (range 0 (Math|Float|Truncate (/ (Variables|Default|GetRangeX) (Variables|Default|GetDistanceBetweenForceLines))))
      (for _index_2 (range 0 (Math|Float|Truncate (/ (Variables|Default|GetRangeY) (Variables|Default|GetDistanceBetweenForceLines))))
        (bind (_outhit _returnvalue_3) (Collision|LineTraceByChannel (Math|Transform|TransformLocation _returnvalue (Math|Vector|MakeVector (- (/ (Variables|Default|GetRangeX) 2.0) (* _index_2 _distancebetweenforcelines)) (- (/ (Variables|Default|GetRangeY) 2.0) (* _index _distancebetweenforcelines)) 0.0)) (Math|Transform|TransformLocation _returnvalue (+ (Math|Vector|MakeVector (- (/ (Variables|Default|GetRangeX) 2.0) (* _index_2 _distancebetweenforcelines)) (- (/ (Variables|Default|GetRangeY) 2.0) (* _index _distancebetweenforcelines)) 0.0) (Math|Vector|MakeVector 0.0 0.0 (Variables|Default|GetRangeZ)))) "TraceTypeQuery1" false 0 "None"))
        (if _returnvalue_3
          (if (Physics|IsSimulatingPhysics (.HitComponent (Collision|BreakHitResult _outhit)) "None")
            (Class|PrimitiveComponent|AddForceatLocation (.HitComponent (Collision|BreakHitResult _outhit)) (* (Math|Vector|Normalize (+ _returnvalue_2 (Math|Vector|NegateVector (.ImpactNormal (Collision|BreakHitResult _outhit))))) (* (Math|Float|Absolute(Float) (Math|Vector|DotProduct _returnvalue_2 (Math|Vector|NegateVector (.ImpactNormal (Collision|BreakHitResult _outhit))))) (Variables|Default|GetMaxForce))) (.ImpactPoint (Collision|BreakHitResult _outhit)) "None")))))))

(event EventBeginPlay
  ;[1 1 1] (Disabled for now) These pieces of code affect the player in regards to wind, player is "flying" and sprinting doesn't do anything when player is in the wind.
  (bind _asthird_person_character (Utilities|Casting|CastToThirdPersonCharacter (Game|GetPlayerCharacter 0))))

(fn ConstructionScript
  (Components|Box|SetBoxExtent (Variables|Default|GetRange) (Math|Vector|MakeVector (/ (Variables|Default|GetRangeX) 2.0) (/ (Variables|Default|GetRangeY) 2.0) (/ (Variables|Default|GetRangeZ) 2.0)) true)
  (Transformation|SetRelativeLocation (Variables|Default|GetRange) (Math|Vector|MakeVector 0.0 0.0 (.z (Variables|/Script/Engine.BoxComponent|GetBoxExtent (Variables|Default|GetRange)))) false false))