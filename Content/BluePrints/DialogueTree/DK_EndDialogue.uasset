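; Behavior tree task that ends an NPC dialogue and returns control to the player.
; It hides the dialogue widget stored in the blackboard and calls DKEndDialogue on the DK_NPC-AI controller.
; It then hides the mouse cursor, switches to game-only input, re-enables player character input and finishes successfully.
; A failed widget or controller cast stops execution before the task finishes.
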(event EventReceiveExecuteAI
  (params (OwnerController :type AI%20Controller%20Object%20Reference) (ControlledPawn :type Pawn%20Object%20Reference))
  (bind _returnvalue (Game|GetPlayerController 0))
  (bind _aswidget (Utilities|Casting|CastToWidget (Class|BTFunctionLibrary|GetBlackboardValueasObject (Variables|Default|GetBB_DialogueUI))))
  (Widget|SetVisibility _aswidget "Hidden")
  (bind _asdk_npc_ai (Utilities|Casting|CastToDK_NPC-AI OwnerController))
  (Default|DKEndDialogue _asdk_npc_ai)
  (Variables|/Script/Engine.PlayerController|SetbShowMouseCursor _returnvalue false)
  (Input|SetInputModeGameOnly _returnvalue)
  (Input|EnableInput (Game|GetPlayerCharacter 0) _returnvalue)
  (AI|BehaviorTree|FinishExecute true))