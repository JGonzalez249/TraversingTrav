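; DK_BehaviorChange is a behavior tree task in the dialogue tree system that changes an NPC's response.
; On execution it casts the controlled pawn to DK_NPC, copies its Behavior variable into that NPC's DKResponse, and finishes successfully.
; A failed cast stops the event without finishing the task.
; Unconnected, never-run nodes would open the HUD dialogue box, store it in the blackboard, and switch player input to the mouse cursor.
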(event EventReceiveExecuteAI
  (params (OwnerController :type AI%20Controller%20Object%20Reference) (ControlledPawn :type Pawn%20Object%20Reference))
  (bind _asdk_npc (Utilities|Casting|CastToDK_NPC ControlledPawn))
  (bind _output_get (Variables|Default|SetDK_NPC-Pawn _asdk_npc))
  (Variables|/Game/NPC/DK_NPC.DK_NPC_C|SetDK_Response _output_get (Variables|Default|GetBehavior))
  (AI|BehaviorTree|FinishExecute true))