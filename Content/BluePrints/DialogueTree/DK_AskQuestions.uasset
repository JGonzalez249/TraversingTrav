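; Behavior Tree task that asks a dialogue question and waits for the player to pick a response.
; It puts the question text in the dialogue box widget from the Blackboard and adds a response list with one clickable widget per response.
; A click writes the response to a Blackboard key as a string, removes the list and finishes the task successfully.
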(event Custom|DK_ResponseReceived
  (params (DK_ResponseReceived :type Text))
  (Class|BTFunctionLibrary|SetBlackboardValueasString (Variables|Default|GetBB_Response) (Utilities|String|ToString(Text) DK_ResponseReceived))
  (Widget|RemovefromParent (Variables|Default|GetDK_ResponseListUI))
  (AI|BehaviorTree|FinishExecute true))

(event EventReceiveExecuteAI
  (params (OwnerController :type AI%20Controller%20Object%20Reference) (ControlledPawn :type Pawn%20Object%20Reference))
  (bind _asdk_dialogue_box (Utilities|Casting|CastToDK_DialogueBox (Class|BTFunctionLibrary|GetBlackboardValueasObject (Variables|Default|GetBB_DialogueUI))))
  (bind _output_get (Variables|Default|SetDK_DialogueBoxUI _asdk_dialogue_box))
  (Variables|/Game/BluePrints/NewUserInterface/DK_DialogueBox.DK_DialogueBox_C|SetDK_DialogueText _output_get (Variables|Default|GetDK_Question))
  (CallFunction|DKPreparedResponses))

(fn DKPreparedResponses
  (bind _returnvalue (UserInterface|CreateWidget "/Game/BluePrints/DialogueTree/DK_ResponseListUI.DK_ResponseListUI_C"))
  (bind _output_get (Variables|Default|SetDK_ResponseListUI _returnvalue))
  (Class|Overlay|AddChildtoOverlay (Variables|/Game/BluePrints/NewUserInterface/DK_DialogueBox.DK_DialogueBox_C|GetResponseListPanel (Variables|Default|GetDK_DialogueBoxUI)) _output_get)
  (for _array_element (Variables|Default|GetDK_Responses)
    (bind _returnvalue_2 (UserInterface|CreateWidget "/Game/BluePrints/DialogueTree/DK_ResponsesUI.DK_ResponsesUI_C" 0 _array_element))
    (Class|VerticalBox|AddChildtoVerticalBox (Variables|/Game/BluePrints/DialogueTree/DK_ResponseListUI.DK_ResponseListUI_C|GetResponseList (Variables|Default|GetDK_ResponseListUI)) _returnvalue_2)
    (EventDispatchers|BindEventtoDKResponseClicked _returnvalue_2 (EventDispatchers|CreateEvent :!event Custom|DK_ResponseReceived))))